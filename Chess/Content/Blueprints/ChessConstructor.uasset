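; Chess board actor that builds tiles and starting pieces in its construction script and handles click-to-move play.
; Pieces live in mesh, type and side maps keyed by a 0-63 square index converted from world positions.
; The first click highlights legal squares; a click on one restores tiles, removes any captured piece and moves the selection.
; Move generation covers only pawn (forward only), rook and king, without turn or check rules.
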(event EventBeginPlay)

(event Collision|EventActorBeginOverlap
  (params (OtherActor :type Actor%20Object%20Reference)))

(event EventTick
  (params (DeltaSeconds :type Float%20%28single-precision%29)))

(fn ConstructionScript
  (bind _chesspieces_mesh (Variables|Default|GetChessPieces_mesh))
  (bind _chesspieces_type (Variables|Default|GetChessPieces_type))
  (bind _chesspieces_side (Variables|Default|GetChessPieces_side))
  (for _index (range 0 63)
    (Utilities|FlowControl|Sequence
      (:then_0
        (bind _returnvalue (AddComponent|AddStaticMeshComponent false (Math|Conversions|ToTransform(Vector) (Utilities|Index->Vector _index))))
        (Utilities|Array|Add (Variables|Default|Gettiles_mesh) _returnvalue)
        (Rendering|Material|SetMaterial _returnvalue 0 (select (Class|KismetMathLibrary|XORBoolean (Math|Conversions|ToBoolean(Integer) (Math|Integer|%(Integer) _index 2)) (Math|Conversions|ToBoolean(Integer) (Math|Integer|%(Integer) (/ _index 8) 2))) "/Game/Assets/Color_Tiles_2.Color_Tiles_2" "/Game/Assets/Color_Tiles_1.Color_Tiles_1"))
        (Utilities|Array|Add (Variables|Default|Gettiles_material) (select (Class|KismetMathLibrary|XORBoolean (Math|Conversions|ToBoolean(Integer) (Math|Integer|%(Integer) _index 2)) (Math|Conversions|ToBoolean(Integer) (Math|Integer|%(Integer) (/ _index 8) 2))) "/Game/Assets/Color_Tiles_2.Color_Tiles_2" "/Game/Assets/Color_Tiles_1.Color_Tiles_1")))
      (:then_1
        (switch int (Utilities|Array|Get(acopy) (Variables|Default|Getstart_figures) _index)
          (:1
            (bind _returnvalue_2 (AddComponent|AddStaticMeshComponent false (Math|Conversions|ToTransform(Vector) (Utilities|Index->Vector _index))))
            (Rendering|Material|SetMaterial _returnvalue_2 0 (select (> _index 30) "/Game/Assets/Color_Pieces_1.Color_Pieces_1" "/Game/Assets/Color_Pieces_2.Color_Pieces_2"))
            (Utilities|Map|Add _chesspieces_mesh (Utilities|Position->Index (* (Utilities|Index->Vector _index) "100.000000,100.000000, 0")) _returnvalue_2)
            (Utilities|Map|Add _chesspieces_type (Utilities|Position->Index (* (Utilities|Index->Vector _index) "100.000000,100.000000, 0")) "pawn"))
          (:2
            (bind _returnvalue_3 (AddComponent|AddStaticMeshComponent false (Math|Conversions|ToTransform(Vector) (Utilities|Index->Vector _index))))
            (Rendering|Material|SetMaterial _returnvalue_3 0 (select (> _index 30) "/Game/Assets/Color_Pieces_1.Color_Pieces_1" "/Game/Assets/Color_Pieces_2.Color_Pieces_2"))
            (Utilities|Map|Add _chesspieces_mesh (Utilities|Position->Index (* (Utilities|Index->Vector _index) "100.000000,100.000000, 0")) _returnvalue_3)
            (Utilities|Map|Add _chesspieces_type (Utilities|Position->Index (* (Utilities|Index->Vector _index) "100.000000,100.000000, 0")) "rook"))
          (:3
            (bind _returnvalue_4 (AddComponent|AddStaticMeshComponent false (Math|Conversions|ToTransform(Vector) (Utilities|Index->Vector _index))))
            (Rendering|Material|SetMaterial _returnvalue_4 0 (select (> _index 30) "/Game/Assets/Color_Pieces_1.Color_Pieces_1" "/Game/Assets/Color_Pieces_2.Color_Pieces_2"))
            (Utilities|Map|Add _chesspieces_mesh (Utilities|Position->Index (* (Utilities|Index->Vector _index) "100.000000,100.000000, 0")) _returnvalue_4)
            (Utilities|Map|Add _chesspieces_type (Utilities|Position->Index (* (Utilities|Index->Vector _index) "100.000000,100.000000, 0")) "knight"))
          (:4
            (bind _returnvalue_5 (AddComponent|AddStaticMeshComponent false (Math|Conversions|ToTransform(Vector) (Utilities|Index->Vector _index))))
            (Rendering|Material|SetMaterial _returnvalue_5 0 (select (> _index 30) "/Game/Assets/Color_Pieces_1.Color_Pieces_1" "/Game/Assets/Color_Pieces_2.Color_Pieces_2"))
            (Utilities|Map|Add _chesspieces_mesh (Utilities|Position->Index (* (Utilities|Index->Vector _index) "100.000000,100.000000, 0")) _returnvalue_5)
            (Utilities|Map|Add _chesspieces_type (Utilities|Position->Index (* (Utilities|Index->Vector _index) "100.000000,100.000000, 0")) "bishop"))
          (:5
            (bind _returnvalue_6 (AddComponent|AddStaticMeshComponent false (Math|Conversions|ToTransform(Vector) (Utilities|Index->Vector _index))))
            (Rendering|Material|SetMaterial _returnvalue_6 0 (select (> _index 30) "/Game/Assets/Color_Pieces_1.Color_Pieces_1" "/Game/Assets/Color_Pieces_2.Color_Pieces_2"))
            (Utilities|Map|Add _chesspieces_mesh (Utilities|Position->Index (* (Utilities|Index->Vector _index) "100.000000,100.000000, 0")) _returnvalue_6)
            (Utilities|Map|Add _chesspieces_type (Utilities|Position->Index (* (Utilities|Index->Vector _index) "100.000000,100.000000, 0")) "queen"))
          (:6
            (bind _returnvalue_7 (AddComponent|AddStaticMeshComponent false (Math|Conversions|ToTransform(Vector) (Utilities|Index->Vector _index))))
            (Rendering|Material|SetMaterial _returnvalue_7 0 (select (> _index 30) "/Game/Assets/Color_Pieces_1.Color_Pieces_1" "/Game/Assets/Color_Pieces_2.Color_Pieces_2"))
            (Utilities|Map|Add _chesspieces_mesh (Utilities|Position->Index (* (Utilities|Index->Vector _index) "100.000000,100.000000, 0")) _returnvalue_7)
            (Utilities|Map|Add _chesspieces_type (Utilities|Position->Index (* (Utilities|Index->Vector _index) "100.000000,100.000000, 0")) "king")))
        (if (< _index 16)
          (Utilities|Map|Add _chesspieces_side (Utilities|Position->Index (* (Utilities|Index->Vector _index) "100.000000,100.000000, 0")) 0)
          (else
            (Utilities|Map|Add _chesspieces_side (Utilities|Position->Index (* (Utilities|Index->Vector _index) "100.000000,100.000000, 0")) 1)))))))

(fn Click
  (params (position :type Vector))
  (bind _returnvalue (Utilities|Position->Index position))
  (Variables|Default|SetActualClick _returnvalue)
  (if (== (Variables|Default|GetLastClick) -1)
    ;[1 1 1] select piece to move
    (bind _positions (Utilities|ChessPieces->MovablePosition _returnvalue)
      (:NewParam
        (if (!= (Utilities|Array|Length _positions) 0)
          (Utilities|FlowControl|Sequence
            (:then_0
              (Variables|Default|SetLastClick _returnvalue))
            (:then_1
              (for _array_element _positions
                (Rendering|Material|SetMaterial (Utilities|Array|Get(acopy) (Variables|Default|Gettiles_mesh) _array_element) 0 "/Game/Assets/Color_Selection.Color_Selection")))))))
    (elif (!= (Utilities|Array|FindItem (Variables|Default|GetMovablePositions) (Variables|Default|GetActualClick)) -1)
      (for _array_element_2 (Variables|Default|GetMovablePositions)
        ;[1 1 1] clear selections visual
        (Rendering|Material|SetMaterial (Utilities|Array|Get(acopy) (Variables|Default|Gettiles_mesh) _array_element_2) 0 (Utilities|Array|Get(acopy) (Variables|Default|Gettiles_material) _array_element_2)))
      ;[1 1 1] move piece
      (Utilities|FlowControl|Sequence
        (:then_0
          (if (.exist (Utilities|GetChessPiece (Variables|Default|GetLastClick)))
            (Utilities|FlowControl|Sequence
              (:then_0
                (Utilities|DeleteChessPiece (Variables|Default|GetActualClick) true))
              (:then_1
                (Utilities|ChangeChessPiecePosition (Variables|Default|GetLastClick) (Variables|Default|GetActualClick))))))
        (:then_1
          (Variables|Default|SetLastClick -1))))))