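; Player controller for a chess game that hosts or joins two-player sessions and turns mouse clicks into piece moves.
; Host creates a non-LAN session and opens the level as a listen server, while Join runs an open console command with the entered IP.
; Left-click release passes the cursor hit location to the level's ChessConstructor, whose valid results go through MovePiece and MovePieceClient back into it, with debug prints.
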(event Custom|Move%20Piece
  (params (from :type Integer) (to :type Integer))
  (Development|PrintString "Hello")
  (CallFunction|MovePieceClient from to))

(event Custom|Move%20Piece%20Client
  (params (from :type Integer) (to :type Integer))
  (Development|PrintString (Utilities|String|BuildString(Integer) (Utilities|String|ToString(Integer) from) " " to))
  (Default|MovePiece (Variables|Default|GetChessConstructor) from to))

(event Custom|Join
  (params (IP :type Text))
  (if (not (Utilities|Text|TextIsEmpty IP))
    (Development|ExecuteConsoleCommand (Utilities|String|Append "open " (Utilities|String|ToString(Text) IP)) 0)))

(event Custom|Host
  (|Session self 2 false
    (:OnSuccess
      (Game|OpenLevel(byName) "Map_level1" true "listen"))))

(event EventBeginPlay
  (Variables|Default|SetbShowMouseCursor true)
  (bind _outactors (Actor|GetAllActorsOfClass "/Game/Blueprints/ChessConstructor.ChessConstructor_C"))
  (Variables|Default|SetChessConstructor (Utilities|Array|Get(acopy) _outactors)))

(event Input|MouseEvents|LeftMouseButton
  (params (Key :type Key%20Structure :default "None"))
  (:Released
    (bind (_from _to) (Default|Click (Variables|Default|GetChessConstructor) (.Location (Collision|BreakHitResult (.HitResult (Game|Player|GetHitResultUnderCursorbyChannel "TraceTypeQuery1" true))))))
    (if (not (or (and (== _from 0) (== _to 0)) (== _from -1)))
      (CallFunction|MovePiece _from _to))))

(fn ConstructionScript)