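; BP_Player is the player pawn Blueprint that handles basic movement and camera look through legacy axis input mappings.
; MoveFront and MoveSide add movement input along the forward and right vectors of the full control rotation, pitch included.
; LookSide and LookFront feed controller yaw and pitch, so looking around also steers the movement direction.
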(event Input|AxisEvents|InputAxisMoveFront
  (params (AxisValue :type Float%20%28single-precision%29))
  ;[1 1 1] Move front or back
  (Pawn|Input|AddMovementInput (Math|Vector|GetForwardVector (Pawn|GetControlRotation :!class /Script/Engine.Pawn)) AxisValue false))

(event Input|AxisEvents|InputAxisMoveSide
  (params (AxisValue :type Float%20%28single-precision%29))
  ;[1 1 1] Move left or right
  (Pawn|Input|AddMovementInput (Math|Vector|GetRightVector (Pawn|GetControlRotation :!class /Script/Engine.Pawn)) AxisValue false))

(event Input|AxisEvents|InputAxisLookSide
  (params (AxisValue :type Float%20%28single-precision%29))
  ;[1 1 1] Move camera
  (Pawn|Input|AddControllerYawInput AxisValue))

(event Input|AxisEvents|InputAxisLookFront
  (params (AxisValue :type Float%20%28single-precision%29))
  ;[1 1 1] Move camera
  (Pawn|Input|AddControllerPitchInput AxisValue))

(fn ConstructionScript)